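; BP_Platform is a moving platform that travels between its spawn location and an offset from it.
; BeginPlay stores the actor location as StartPoint and plays a timeline.
; Each timeline update lerps the Platform component's world location from StartPoint to StartPoint plus EndPoint, without sweep.
; An older start and end location setup remains in the graph but never runs.
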(event EventBeginPlay
  (Variables|Default|SetStartPoint (Transformation|GetActorLocation))
  (bind _newtrack_0 (Timeline|Timeline_0 Play)
    (:Update
      (Transformation|SetWorldLocation (Variables|Default|GetPlatform) (Math|Vector|Lerp(Vector) (Variables|Default|GetStartPoint) (+ (Variables|Default|GetStartPoint) (Variables|Default|GetEndPoint)) _newtrack_0) false false))))

(fn ConstructionScript)