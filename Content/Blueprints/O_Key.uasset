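; O_Key is a collectible key pickup that spins around its roll axis every tick.
; Any overlap with its Box plays a sound, then adds its Key value to the player pawn's WRONG_CHARACTER and destroys the actor.
; The cast targets player pawn 0, not the overlapping actor.
; The construction script loops to add child actor components at the Box's relative location, as the random-point extent is zero.
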(event OnComponentBeginOverlap(Box)
  (params (OverlappedComponent :type Primitive%20Component%20Object%20Reference) (OtherActor :type Actor%20Object%20Reference) (OtherComp :type Primitive%20Component%20Object%20Reference) (OtherBodyIndex :type Integer) (bFromSweep :type Boolean) (SweepResult :type Hit%20Result%20Structure%20%28by%20ref%29))
  (Audio|PlaySound2D 0 1.0 1.0 0.0 0 0)
  (bind _aswrong_character (Utilities|Casting|CastToWRONG_CHARACTER (Game|Player|GetPlayerPawn 0)))
  (Variables|/Game/ThirdPersonBP/Blueprints/WRONG_CHARACTER.WRONG_CHARACTER_C|SetKey _aswrong_character (+ (Variables|/Game/ThirdPersonBP/Blueprints/WRONG_CHARACTER.WRONG_CHARACTER_C|GetKey _aswrong_character) (Variables|Default|GetKey)))
  (Actor|DestroyActor))

(event EventTick
  (params (DeltaSeconds :type Float%20%28single-precision%29))
  (bind _0_key (Variables|Default|Get0_Key))
  (bind _relativerotation (Variables|/Script/Engine.SceneComponent|GetRelativeRotation _0_key))
  (Transformation|SetRelativeRotation _0_key (Math|Rotator|MakeRotator (+ (.roll _relativerotation) 1.0) (.pitch _relativerotation) (.yaw _relativerotation)) false false))

(fn ConstructionScript
  (CallFunction|SpawnOKey))

(fn SpawnOKey
  (for _index (range 0 1)
    (AddComponent|AddChildActorComponent false (Math|Conversions|ToTransform(Vector) (Math|Random|RandomPointinBoundingBox (Variables|/Script/Engine.SceneComponent|GetRelativeLocation (Variables|Default|GetBox)) "0, 0, 0")))))